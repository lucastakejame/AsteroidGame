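; BP_CanvasDrawer paints Bokeh sprites onto a render target in the Asteroids game.
; DrawAtLocation maps a world location onto the canvas and additively stamps a randomly sized, tinted spot.
; A looping BeginPlay timer darkens the target through a Modulate pass while IsFadingColors is set, fading earlier marks.
; RandomPainting copies the AnalogHat texture to a temporary target, then repeatedly scatters small dots colored from its sampled pixels.
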(event Custom|DrawToCanvas
  (bind (_canvas _size _context) (Rendering|BeginDrawCanvastoRenderTarget (Variables|Default|GetrenderTarget)))
  (Canvas|DrawTexture _canvas "/Engine/Engine_MI_Shaders/Textures/Bokeh.Bokeh" (Variables|Default|GetscreenPosition) (Variables|Default|GetscreenSize) (Variables|Default|GetcoordinatePosition) (Variables|Default|GetcoordinateSize) (Variables|Default|GetrenderColor) (Variables|Default|GetblendMode) 0.0 (Variables|Default|GetpivotPoint))
  (Rendering|EndDrawCanvastoRenderTarget _context))

(event Custom|ClearCanvas
  (Rendering|ClearRenderTarget2D self (Variables|Default|GetrenderTarget)))

(event Custom|DrawAtLocation
  (params (location :type Vector) (RenderColor :type Linear%20Color%20Structure))
  (bind _returnvalue (Math|Vector2D|MakeVector2D 4.1e+03 2.25e+03))
  (bind (_x _y) (Math|Vector|BreakVector location))
  (bind (_canvas _size _context) (Rendering|BeginDrawCanvastoRenderTarget (Variables|Default|GetrenderTarget)))
  (Variables|Default|SetrandomValue (Math|Random|RandomFloat))
  (Canvas|DrawTexture :self _canvas :RenderTexture "/Engine/Engine_MI_Shaders/Textures/Bokeh.Bokeh" :ScreenPosition (- (* _size (/ (+ (Math|Vector2D|MakeVector2D _y (* _x -1.0)) (/ _returnvalue 2.0)) _returnvalue)) (/ (Math|Vector2D|MakeVector2D (Math|Float|MakeLiteralFloat (Math|Float|Lerp 2e+01 2e+02 (Variables|Default|GetrandomValue))) (Math|Float|MakeLiteralFloat (Math|Float|Lerp 2e+01 2e+02 (Variables|Default|GetrandomValue)))) 2.0)) :ScreenSize (Math|Vector2D|MakeVector2D (Math|Float|MakeLiteralFloat (Math|Float|Lerp 2e+01 2e+02 (Variables|Default|GetrandomValue))) (Math|Float|MakeLiteralFloat (Math|Float|Lerp 2e+01 2e+02 (Variables|Default|GetrandomValue)))) :RenderColor RenderColor :BlendMode "BLEND_Additive" :PivotPoint "(X=0.000000,Y=0.000000)")
  (Rendering|EndDrawCanvastoRenderTarget _context))

(event Custom|DarkenCanvas
  (bind _returnvalue (Math|Float|MakeLiteralFloat 1.5))
  (if (Variables|Default|GetisFadingColors)
    (bind (_canvas _size _context) (Rendering|BeginDrawCanvastoRenderTarget (Variables|Default|GetrenderTarget)))
    (Canvas|DrawTexture :self _canvas :RenderTexture "/Engine/ArtTools/RenderToTexture/Textures/127grey.127grey" :ScreenSize _size :RenderColor (Math|Color|MakeColor _returnvalue _returnvalue _returnvalue) :BlendMode "BLEND_Modulate" :PivotPoint "(X=0.000000,Y=0.000000)")
    (Rendering|EndDrawCanvastoRenderTarget _context)))

(event Custom|RandomPainting
  ;[1 1 1] Paint texture with dots
  (Utilities|Time|SetTimerbyEvent (delegate Custom|PaintRandomSpot) (Utilities|Time|GetWorldDeltaSeconds) true)
  (bind _returnvalue (CanvasRenderTarget2D|CreateCanvasRenderTarget2D "/Script/Engine.CanvasRenderTarget2D" 1024 1024))
  (CallFunction|DrawTexturetoCanvas _returnvalue "/Engine/MobileResources/HUD/AnalogHat.AnalogHat"))

(event Custom|PaintRandomSpot
  (bind _returnvalue (Math|Float|MakeLiteralFloat 1e+01))
  ;[1 1 1] Paint texture with dots
  (bind (_canvas _size _context) (Rendering|BeginDrawCanvastoRenderTarget (Variables|Default|GetrenderTarget)))
  (Utilities|FlowControl|Sequence
    (:then_0
      (for _index (range 0 100)
        (bind _returnvalue_2 (Class|KismetRenderingLibrary|ReadRenderTargetPixel (stale Custom|RandomPainting _returnvalue) (Math|Float|Truncate (* 1024 (/ (Math|Float|Lerp 0.0 (.X (Math|Vector2D|BreakVector2D _size)) (Math|Random|RandomFloat)) (.X (Math|Vector2D|BreakVector2D _size))))) (Math|Float|Truncate (* 1024 (/ (Math|Float|Lerp 0.0 (.Y (Math|Vector2D|BreakVector2D _size)) (Math|Random|RandomFloat)) (.Y (Math|Vector2D|BreakVector2D _size)))))))
        (Canvas|DrawTexture :self _canvas :RenderTexture "/Engine/Engine_MI_Shaders/Textures/Bokeh.Bokeh" :ScreenPosition (Math|Vector2D|MakeVector2D (Math|Float|Lerp 0.0 (.X (Math|Vector2D|BreakVector2D _size)) (Math|Random|RandomFloat)) (Math|Float|Lerp 0.0 (.Y (Math|Vector2D|BreakVector2D _size)) (Math|Random|RandomFloat))) :ScreenSize (Math|Vector2D|MakeVector2D _returnvalue _returnvalue) :RenderColor (Math|Conversions|ToLinearColor(Color) _returnvalue_2) :BlendMode "BLEND_Masked" :PivotPoint "(X=0.000000,Y=0.000000)")))
    (:then_1
      (Rendering|EndDrawCanvastoRenderTarget _context))))

(event Custom|DrawTextureToCanvas
  (params (TextureRenderTarget :type Texture%20Render%20Target%202D%20Object%20Reference) (RenderTexture :type Texture%20Object%20Reference))
  (bind (_canvas _size _context) (Rendering|BeginDrawCanvastoRenderTarget TextureRenderTarget))
  (Canvas|DrawTexture :self _canvas :RenderTexture RenderTexture :ScreenSize _size :BlendMode "BLEND_Additive" :PivotPoint "(X=0.000000,Y=0.000000)")
  (Rendering|EndDrawCanvastoRenderTarget _context))

(event EventBeginPlay
  (Utilities|Time|SetTimerbyEvent (delegate Custom|DarkenCanvas) 0.1 true))

(fn ConstructionScript)