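; BP_BlackHole is a black hole for the Asteroids game that pulls in and swallows other actors.
; A looping timer caches all actors tagged "wrappable", and Tick offsets each toward the hole by inverse-square attraction from its squared Strength, unscaled by delta time.
; Each pull draws a debug line.
; Mesh hits from anything except Projectile destroy that actor, raise Strength and enlarge the mesh by the victim's bounds.
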(event OnComponentHit(StaticMesh)
  (params (HitComponent :type Primitive%20Component%20Object%20Reference) (OtherActor :type Actor%20Object%20Reference) (OtherComp :type Primitive%20Component%20Object%20Reference) (NormalImpulse :type Vector :default "0, 0, 0") (Hit :type Hit%20Result%20Structure%20%28by%20ref%29))
  (if (not (== (Utilities|GetClass OtherActor) "/Script/portifolio.Projectile"))
    (Utilities|FlowControl|DoOnce false :!label _label
      (:Completed
        (Variables|Default|Setstrength (+ (Variables|Default|Getstrength) 5e+01))
        (Transformation|SetWorldScale3D (Variables|Default|GetStaticMesh) (+ (Transformation|GetWorldScale (Variables|Default|GetStaticMesh)) (Math|Conversions|ToVector(Float) (/ (Math|Vector|GetMaxElement (.BoxExtent (Collision|GetActorBounds OtherActor false))) 2e+02))))
        (Actor|DestroyActor OtherActor)
        (goto _label Reset)))))

(event Custom|GatherActors
  (bind _outactors (Actor|GetAllActorswithTag "wrappable"))
  (Variables|Default|Setactors _outactors))

(event EventBeginPlay
  (Utilities|Time|SetTimerbyEvent (delegate Custom|GatherActors) 0.2 true))

(event EventTick
  (params (DeltaSeconds :type Float%20%28single-precision%29))
  (bind _strength (Variables|Default|Getstrength))
  (for _array_element (Variables|Default|Getactors)
    (Utilities|IsValid _array_element
      (:Is%20Valid
        (Transformation|SetActorLocation _array_element (+ (Transformation|GetActorLocation _array_element) (/ (* (Math|Vector|Normalize (- (Transformation|GetActorLocation) (Transformation|GetActorLocation _array_element))) (* _strength _strength)) (Math|Vector|VectorLengthSquared (- (Transformation|GetActorLocation) (Transformation|GetActorLocation _array_element))))) false false)
        (Rendering|Debug|DrawDebugLine (Transformation|GetActorLocation) (+ (Transformation|GetActorLocation _array_element) (/ (* (Math|Vector|Normalize (- (Transformation|GetActorLocation) (Transformation|GetActorLocation _array_element))) (* _strength _strength)) (Math|Vector|VectorLengthSquared (- (Transformation|GetActorLocation) (Transformation|GetActorLocation _array_element))))) "(R=1.000000,G=1.000000,B=1.000000,A=1.000000)" 0.0 4.0)))))

(fn ConstructionScript)