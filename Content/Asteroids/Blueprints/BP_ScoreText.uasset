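; Floating score text actor for the Asteroids game that shows its Text value as a short animated pop-up, then removes itself.
; On BeginPlay it pitches the text upward with a randomized yaw and sets the string.
; A sped-up timeline lerps the text along the actor's up vector from its starting location while growing its size, then a near-zero lifespan destroys the actor when it finishes.
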(event EventBeginPlay
  (bind _returnvalue (Transformation|GetActorUpVector))
  (bind _textrender (Variables|Default|GetTextRender))
  (Variables|Default|SetreferenceLocation (Transformation|GetActorLocation))
  (Transformation|SetWorldRotation _textrender (Math|Rotator|MakeRotator 0.0 9e+01 (Math|Float|Lerp 1.5e+02 2.3e+02 (Math|Random|RandomFloat))) false false)
  (Rendering|Components|TextRender|SetText _textrender (Variables|Default|Gettext))
  (Components|Timeline|SetPlayRate (Variables|Default|GetTL_TextMovement) (/ 1.0 0.5))
  (bind _movementprogress (Timeline|TL_TextMovement PlayFromStart)
    (:Update
      (Transformation|SetWorldLocation _textrender (Math|Vector|Lerp(Vector) (+ (Variables|Default|GetreferenceLocation) (* _returnvalue 5e+01)) (+ (Variables|Default|GetreferenceLocation) (* _returnvalue 8e+01)) _movementprogress) false false)
      (Rendering|Components|TextRender|SetWorldSize _textrender (Math|Float|Lerp 1e+02 1.5e+02 _movementprogress)))
    (:Finished
      (Actor|SetLifeSpan 0.001))))

(fn ConstructionScript)