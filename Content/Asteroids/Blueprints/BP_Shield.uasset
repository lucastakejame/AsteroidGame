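; BP_Shield is a shield pickup in the Asteroids game that protects the affected pawn and damages what hits it.
; ApplyEffect stores and attaches to the pawn, clears the lifespan, hides the pickup mesh and disables its collision, then shows MeshShield with the Player collision profile.
; Shield hits send fixed damage through DamageInterface to implementing actors, crediting the owning pawn as instigator.
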(event OnComponentHit(MeshShield)
  (params (HitComponent :type Primitive%20Component%20Object%20Reference) (OtherActor :type Actor%20Object%20Reference) (OtherComp :type Primitive%20Component%20Object%20Reference) (NormalImpulse :type Vector :default "0, 0, 0") (Hit :type Hit%20Result%20Structure%20%28by%20ref%29))
  (if (Utilities|DoesObjectImplementInterface OtherActor "/Script/portifolio.DamageInterface")
    (Class|DamageInterface|ReceiveDamage(Message) OtherActor (Variables|Default|GetOwnerPawn) 3e+01)))

(event EventApplyEffect
  (params (pAffectedPawn :type Pawn%20Object%20Reference))
  (bind _mpmeshcomponent (Variables|Default|GetmpMeshComponent))
  (Variables|Default|SetOwnerPawn pAffectedPawn)
  (Transformation|AttachActorToActor pAffectedPawn "None" "SnapToTarget" "SnapToTarget" "KeepWorld" true)
  (Actor|SetLifeSpan 0.0)
  (Utilities|FlowControl|Sequence
    (:then_0
      (Rendering|SetVisibility _mpmeshcomponent false false)
      (Collision|SetCollisionEnabled _mpmeshcomponent "NoCollision"))
    (:then_1
      (Development|SetHiddeninGame (Variables|Default|GetMeshShield) false false)
      (Collision|SetCollisionProfileName (Variables|Default|GetMeshShield) "Player" :!class /Script/Engine.PrimitiveComponent))))

(fn ConstructionScript)