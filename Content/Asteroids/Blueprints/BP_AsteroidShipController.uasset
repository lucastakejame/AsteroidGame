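; Player controller for the Asteroids game that routes input to either the player's ship or menu navigation.
; On BeginPlay it caches the ship pawn and the Asteroids game mode, then enables input.
; The game mode's menu state gates each input: gameplay drives movement, shooting and quick turns on the ship, while menus get cursor and confirm calls, with Shoot doubling as confirm.
; Pause toggles through the game mode in either state.
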(event EventBeginPlay
  (Utilities|FlowControl|Sequence
    (:then_0
      (bind _asasteroid_ship (Utilities|Casting|CastToAsteroidShip (Game|Player|GetPlayerPawn 0)))
      (Variables|Default|SetshipRef _asasteroid_ship)
      (Input|EnableInput self))
    (:then_1
      (bind _asbp_asteroid_game_mode (Utilities|Casting|CastToBP_AsteroidGameMode (Game|GetGameMode)))
      (Variables|Default|SetGameModeRef _asbp_asteroid_game_mode))))

(event Input|ActionEvents|InputActionShoot
  (params (Key :type Key%20Structure))
  (bind _shipref (Variables|Default|GetshipRef))
  (:Pressed
    (if (Default|IsMenuMode (Variables|Default|GetGameModeRef))
      ;[1 1 1] Cursor events
      (Default|CallOnPressedConfirm)
      (else
        (Class|AsteroidShip|EnableShooting _shipref))))
  (:Released
    (if (not (Default|IsMenuMode (Variables|Default|GetGameModeRef)))
      (Class|AsteroidShip|DisableShooting _shipref))))

(event Input|ActionEvents|InputActionQuickTurn
  (params (Key :type Key%20Structure))
  (:Pressed
    (if (not (Default|IsMenuMode (Variables|Default|GetGameModeRef)))
      (Class|AsteroidShip|TurnQuickly (Variables|Default|GetshipRef)))))

(event Input|ActionEvents|InputActionCursorDown
  (params (Key :type Key%20Structure))
  ;[1 1 1] Cursor events
  (:Pressed
    (if (Default|IsMenuMode (Variables|Default|GetGameModeRef))
      (Default|CallOnPressedDown))))

(event Input|ActionEvents|InputActionCursorUp
  (params (Key :type Key%20Structure))
  ;[1 1 1] Cursor events
  (:Pressed
    (if (Default|IsMenuMode (Variables|Default|GetGameModeRef))
      (Default|CallOnPressedUp))))

(event Input|ActionEvents|InputActionPause
  (params (Key :type Key%20Structure))
  (:Pressed
    (Default|TogglePause (Variables|Default|GetGameModeRef))))

(event Input|ActionEvents|InputActionCursorRight
  (params (Key :type Key%20Structure))
  ;[1 1 1] Cursor events
  (:Pressed
    (if (Default|IsMenuMode (Variables|Default|GetGameModeRef))
      (Default|CallOnPressedRight))))

(event Input|ActionEvents|InputActionCursorLeft
  (params (Key :type Key%20Structure))
  ;[1 1 1] Cursor events
  (:Pressed
    (if (Default|IsMenuMode (Variables|Default|GetGameModeRef))
      (Default|CallOnPressedLeft))))

(event Input|AxisEvents|InputAxisMoveForward
  (params (AxisValue :type Float%20%28single-precision%29))
  (if (not (Default|IsMenuMode (Variables|Default|GetGameModeRef)))
    (Class|AsteroidShip|SetForwardValue (Variables|Default|GetshipRef) AxisValue)))

(event Input|AxisEvents|InputAxisMoveRight
  (params (AxisValue :type Float%20%28single-precision%29))
  (if (not (Default|IsMenuMode (Variables|Default|GetGameModeRef)))
    (Class|AsteroidShip|SetRotatingValue (Variables|Default|GetshipRef) AxisValue)))

(fn ConstructionScript)