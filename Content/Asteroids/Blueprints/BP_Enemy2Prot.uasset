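; BP_Enemy2Prot is an enemy in the Asteroids game that chases the player's ship when it is nearby.
; BeginPlay caches the player pawn as BP_AsteroidShip and starts a short looping timer that calls ThrustToPawn.
; Within a fixed range, ThrustToPawn overwrites the mesh's physics velocity toward the ship, using MLimitSpeed multiplied by mass rather than applying a force.
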(event Custom|ThrustToPawn
  (bind _returnvalue (Transformation|GetActorLocation))
  (bind _playerref (Variables|Default|GetplayerRef))
  (bind _mlimitspeed (Variables|Default|GetmLimitSpeed))
  (bind _returnvalue_2 (Transformation|GetActorLocation _playerref))
  (bind _returnvalue_3 (- _returnvalue_2 _returnvalue))
  (if (<= (Math|Vector|VectorLength _returnvalue_3) 8e+02)
    (Physics|SetPhysicsLinearVelocity (Variables|Default|GetmpMeshComponent) (* (Math|Vector|ClampVectorSize _returnvalue_3 _mlimitspeed _mlimitspeed) (Physics|GetMass (Variables|Default|GetmpMeshComponent))) false "None")))

(event EventBeginPlay
  (Utilities|FlowControl|Sequence
    (:then_0
      (bind _asbp_asteroid_ship (Utilities|Casting|CastToBP_AsteroidShip (Game|Player|GetPlayerPawn 0)))
      (Variables|Default|SetplayerRef _asbp_asteroid_ship))
    (:then_1
      (Utilities|Time|SetTimerbyEvent (delegate Custom|ThrustToPawn) 0.3 true))))

(fn ConstructionScript)