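; Game mode for the Asteroids game that runs the start, pause and after-death menu and broadcasts game start and end.
; BeginPlay binds to the player ship's lives-ended event and pauses; pausing shows a lazily created, reused W_Menu, whose button resumes play.
; When lives end, it announces game over and shows the menu after a delay without pausing.
; A flag makes that button restart without toggling pause.
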(event Custom|HandlePlayerLivesEnding
  (Variables|Default|SetisStartMenu true)
  (Default|CallMonGameEnded)
  (Utilities|FlowControl|Delay 4.0)
  (CallFunction|AddMenutoScreenandSetDelegate (Variables|Default|GetMenuRef))
  (Variables|Default|SetisAfterDeathMenu true))

(event Custom|StartOrResumeButtonPressed
  (if (Variables|Default|GetisAfterDeathMenu)
    (Variables|Default|SetisAfterDeathMenu false)
    (CallFunction|RemoveMenufromScreen)
    (else
      (CallFunction|TogglePause)))
  (Utilities|IsValid (Variables|Default|GetMenuRef)
    (:Is%20Valid
      (EventDispatchers|UnbindEventfromOnStartGamePressed (Variables|Default|GetMenuRef) (delegate Custom|StartOrResumeButtonPressed)))))

(event Custom|TogglePause
  (CallFunction|SetGamePaused (not (Game|IsGamePaused))))

(event Custom|AddMenuToScreenAndSetDelegate
  (params (menuWidget :type W%20Menu%20Object%20Reference))
  (EventDispatchers|BindEventtoOnStartGamePressed menuWidget (delegate Custom|StartOrResumeButtonPressed))
  (Default|ChangeGameStartText menuWidget (Variables|Default|GetisStartMenu))
  (UserInterface|Viewport|AddtoPlayerScreen menuWidget))

(event Custom|SetGamePaused
  (params (isPaused :type Boolean))
  (Game|SetGamePaused isPaused)
  (if isPaused
    (CallFunction|AddMenutoScreen)
    (else
      (CallFunction|RemoveMenufromScreen))))

(event Custom|AddMenuToScreen
  (Utilities|IsValid (Variables|Default|GetMenuRef)
    (:Is%20Valid
      _)
    (:Is%20Not%20Valid
      (bind _returnvalue (UserInterface|CreateWidget "/Game/Asteroids/Widgets/W_Menu.W_Menu_C" (Game|GetPlayerController 0)))
      (Variables|Default|SetMenuRef _returnvalue)))
  (CallFunction|AddMenutoScreenandSetDelegate (Variables|Default|GetMenuRef)))

(event Custom|RemoveMenuFromScreen
  (if (Variables|Default|GetisStartMenu)
    (Default|CallMonGameStarted)
    (Variables|Default|SetisStartMenu false))
  (Widget|RemovefromParent (Variables|Default|GetMenuRef)))

(event EventBeginPlay
  (|ReferenceAndBindings)
  (CallFunction|TogglePause))

(fn ConstructionScript)

(fn IsMenuMode
  (return (or (Game|IsGamePaused) (Variables|Default|GetisAfterDeathMenu))))