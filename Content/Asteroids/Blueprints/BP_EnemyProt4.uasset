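; BP_EnemyProt4 is a prototype Asteroids enemy that forms a pair of actors orbiting their shared midpoint.
; The dominant instance spawns and re-materials itself, then each tick pushes the center, speed and radius to its non-dominant partner.
; A real-time sine, squared, pulses the radius, while a power curve spins the pair faster as they draw closer.
; Both rotate around Z by a per-frame angle, not scaled by delta time.
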(event EventTick
  (params (DeltaSeconds :type Float%20%28single-precision%29))
  (Utilities|FlowControl|Sequence
    (:then_0
      (if (Variables|Default|GetisDominant)
        (bind _output_get (Variables|Default|SetorbitCenter (/ (+ (Transformation|GetActorLocation (Variables|Default|GetOther)) (Transformation|GetActorLocation) "0,0.000000,0") 2.0)))
        (Variables|BP_EnemyProt4_C|SetorbitCenter (Variables|Default|GetOther) _output_get)
        (bind _output_get_2 (Variables|Default|SetorbSpeed (Math|Float|Lerp 5.0 4e+01 (Math|Float|Power (Math|Float|MapRangeClamped (Math|Vector|VectorLength (- (Transformation|GetActorLocation) (Variables|Default|GetorbitCenter))) 1e+02 313.0 1.0 0.0) 4.0))))
        (Variables|BP_EnemyProt4_C|SetorbSpeed (Variables|Default|GetOther) _output_get_2)
        (bind _output_get_3 (Variables|Default|SetdistFromCenter (Math|Float|Square (Math|Float|MapRangeClamped (Math|Trig|Sin(Radians) (Utilities|Time|GetRealTimeSeconds)) -1.0 1.0 1e+01 18.0))))
        (Variables|BP_EnemyProt4_C|SetdistFromCenter (Variables|Default|GetOther) _output_get_3)))
    (:then_1
      (Transformation|SetActorLocationAndRotation (+ (Variables|Default|GetorbitCenter) (Math|Vector|ClampVectorSize (Math|Vector|RotateVectorAroundAxis (- (Transformation|GetActorLocation) (Variables|Default|GetorbitCenter)) (Variables|Default|GetorbSpeed) "0, 0,1.000000") (Variables|Default|GetdistFromCenter) (Variables|Default|GetdistFromCenter))) "0, 0, 0"))))

(event EventBeginPlay
  (bind _self self)
  (if (Variables|Default|GetisDominant)
    (bind _returnvalue (Game|SpawnActorfromClass "BP_EnemyProt4_C" (Math|Transform|MakeTransform (+ (Transformation|GetActorLocation) "200.000000, 0, 0") "0, 0, 0" "1,1,1") "Undefined" _self _self false 0))
    (Variables|Default|SetOther _returnvalue)
    (Rendering|Material|SetMaterial (Variables|Default|GetmpMeshComponent) 0 "/Engine/MapTemplates/Materials/BasicAsset03.BasicAsset03")))

(fn ConstructionScript)