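; BP_Blade is a melee gun pickup in the Asteroids game that attaches to the player's ship as a swinging blade.
; On pickup it becomes the ship's gun, swaps the pickup mesh for a collidable blade, and hides the blade when the ship loses a life.
; Shooting plays a cooldown-scaled timeline that spins and enlarges it.
; Blade hits knock Targets away and deal damage credited to the owning ship.
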(event OnComponentHit(meshBlade)
  (params (HitComponent :type Primitive%20Component%20Object%20Reference) (OtherActor :type Actor%20Object%20Reference) (OtherComp :type Primitive%20Component%20Object%20Reference) (NormalImpulse :type Vector :default "0, 0, 0") (Hit :type Hit%20Result%20Structure%20%28by%20ref%29))
  (bind _astarget (Utilities|Casting|CastToTarget OtherActor))
  (Physics|AddImpulseatLocation (Variables|/Script/portifolio.Target|GetmpMeshComponent _astarget) (* NormalImpulse 2e+01) (.location Hit) "None")
  (Class|DamageInterface|ReceiveDamage _astarget (.AsBP%20Asteroid%20Ship (Utilities|Casting|CastToBP_AsteroidShip (Components|GetOwner))) 1e+02))

(event Custom|rotateBlade
  (bind (_direction _angleprogress _scaleprogress) (Timeline|TL_Scale PlayFromStart)
    (:Update
      (Transformation|SetRelativeRotation (Variables|Default|GetmpMeshComponent) (Math|Rotator|MakeRotator 0.0 0.0 (Math|Float|Lerp 1.8e+02 -1.8e+02 _angleprogress)) false false)
      (Transformation|SetActorScale3D (Math|Conversions|ToVector(Float) (Math|Float|Lerp 1.0 2.0 _scaleprogress))))))

(event Custom|SetBladeInvisible
  (Development|SetHiddeninGame (Variables|Default|GetmeshBlade) true false))

(event EventBeginPlay
  (Components|Timeline|SetPlayRate (Variables|Default|GetTL_Scale) (/ 1.0 (* (Variables|Default|GetmShootCoolDown) 0.9))))

(event EventApplyEffect
  (params (pAffectedPawn :type Pawn%20Object%20Reference))
  (bind _asbp_asteroid_ship (Utilities|Casting|CastToBP_AsteroidShip pAffectedPawn))
  (Actor|SetOwner _asbp_asteroid_ship)
  (Transformation|AttachActorToActor _asbp_asteroid_ship "None" "SnapToTarget" "SnapToTarget" "KeepWorld" true)
  (Actor|SetLifeSpan 0.0)
  (Class|AsteroidShip|SetGun _asbp_asteroid_ship self)
  (Development|SetHiddeninGame (Variables|Default|GetmpMeshComponent) true false)
  (Development|SetHiddeninGame (Variables|Default|GetmeshBlade) false false)
  (Collision|SetCollisionEnabled (Variables|Default|GetmeshBlade) "QueryAndPhysics")
  (Transformation|SetRelativeRotation (Variables|Default|GetmpMeshComponent) (Math|Rotator|MakeRotator 0.0 0.0 1.8e+02) false false)
  (EventDispatchers|BindEventtoMonLosingLife _asbp_asteroid_ship (delegate Custom|SetBladeInvisible)))

(event EventShoot
  (if (Variables|Default|GetmCanShoot)
    (Variables|Default|SetmCanShoot false)
    (Utilities|FlowControl|Sequence
      (:then_0
        (Utilities|FlowControl|Delay (Variables|Default|GetmShootCoolDown))
        (Variables|Default|SetmCanShoot true))
      (:then_1
        (CallFunction|RotateBlade)))))

(fn ConstructionScript
  (Collision|SetCollisionEnabled (Variables|Default|GetmeshBlade) "NoCollision"))