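; Player ship Blueprint for an Asteroids game, adding HUD, new-game reset and thruster effects to its parent class.
; On BeginPlay it creates the HUD widget, binds to the game mode's game-started delegate, shows the HUD and enables input.
; A StartNewGame event resets the ship to its begin state.
; The MoveForward axis magnitude is remapped to the Niagara spawn rate, so particle emission scales with thrust input.
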(event Custom|StartNewGame
  (Class|AsteroidShip|ResetShiptoBeginState))

(event EventBeginPlay
  (|CallParentFunction)
  (|ReferencesAndBinding)
  (UserInterface|Viewport|AddtoViewport (Variables|Default|GetHUDWidgetRef) 0)
  (Input|EnableInput (Game|GetPlayerController 0)))

(event Input|AxisEvents|InputAxisMoveForward
  (params (AxisValue :type Float%20%28single-precision%29))
  (Niagara|SetNiagaraVariable(Float) (Variables|Default|GetNiagara) "User.SpawnRate" (Math|Float|MapRangeClamped (Math|Float|Absolute(Float) AxisValue) 0.1 1.0 0.0 3e+02)))

(fn ConstructionScript)