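; Game instance for the Asteroids game that persists audio volume settings and applies them through sound mixes.
; On Init it loads or creates a config save object, pushes the music and SFX mixes after a short delay, and applies the saved volumes without waiting for that delay.
; Volume setters clamp the value, store it in the config and override the sound class volume.
; Shutdown writes the config to its slot.
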(event Custom|SetSFXVolume
  (params (Volume :type Float%20%28single-precision%29))
  (bind _output_get (Variables|/Game/Asteroids/Blueprints/BP_SaveAsteroidConfig.BP_SaveAsteroidConfig_C|SetVolumeSFX (Variables|Default|GetsaveConfig) (Math|Float|Clamp(Float) Volume 0.01)))
  (Audio|SetSoundMixClassOverride (Game|Player|GetPlayerPawn 0) (Variables|Default|GetSMXSFX) "/Engine/EngineSounds/SFX.SFX" _output_get 1.0 0.2 true))

(event Custom|SetMusicVolume
  (params (Volume :type Float%20%28single-precision%29))
  (bind _output_get (Variables|/Game/Asteroids/Blueprints/BP_SaveAsteroidConfig.BP_SaveAsteroidConfig_C|SetVolumeMusic (Variables|Default|GetsaveConfig) (Math|Float|Clamp(Float) Volume)))
  (Audio|SetSoundMixClassOverride (Game|Player|GetPlayerPawn 0) (Variables|Default|GetSMXMusic) "/Engine/EngineSounds/Music.Music" _output_get 1.0 0.2 true))

(event EventInit
  (Utilities|FlowControl|Sequence
    (:then_0
      (bind _savegame (CallFunction|LoadorCreateGameSlot "config.slot"))
      (Variables|Default|SetsaveConfig _savegame))
    (:then_1
      ;[1 1 1] Enabling mixes
      (Utilities|FlowControl|Delay 0.2)
      (Audio|PushSoundMixModifier "/Game/Asteroids/Sounds/SMX_Music.SMX_Music")
      (Audio|PushSoundMixModifier "/Game/Asteroids/Sounds/SMX_SFX.SMX_SFX"))
    (:then_2
      ;[1 1 1] Setting Defaults
      (CallFunction|SetMusicVolume (Variables|/Game/Asteroids/Blueprints/BP_SaveAsteroidConfig.BP_SaveAsteroidConfig_C|GetVolumeMusic (Variables|Default|GetsaveConfig)))
      (CallFunction|SetSFXVolume (Variables|/Game/Asteroids/Blueprints/BP_SaveAsteroidConfig.BP_SaveAsteroidConfig_C|GetVolumeSFX (Variables|Default|GetsaveConfig))))))

(event EventShutdown
  (SaveGame|SaveGametoSlot (Variables|Default|GetsaveConfig) "config.slot"))

(fn LoadorCreateGameSlot
  (params (loadSlotName :type String))
  (LocalVariables|SetslotName loadSlotName)
  (bind _returnvalue (SaveGame|DoesSaveGameExist (LocalVariables|GetslotName)))
  (if _returnvalue
    (bind _returnvalue_2 (SaveGame|LoadGamefromSlot (LocalVariables|GetslotName)))
    (bind _asbp_save_asteroid_config (Utilities|Casting|CastToBP_SaveAsteroidConfig _returnvalue_2))
    (return _asbp_save_asteroid_config)
    (else
      (bind _returnvalue_3 (SaveGame|CreateSaveGameObject "/Game/Asteroids/Blueprints/BP_SaveAsteroidConfig.BP_SaveAsteroidConfig_C"))
      (SaveGame|SaveGametoSlot _returnvalue_3 (LocalVariables|GetslotName))
      (return _returnvalue_3))))